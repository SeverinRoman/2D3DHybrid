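; UI manager actor that puts configured screen widgets on the viewport when play begins.
; On BeginPlay it prints the platform name, toggles one extra screen type on Android, then toggles every ScreenConfigs entry flagged IsStart.
; ToggleUI creates and adds a new widget for each config matching the screen type.
; Its IsOn input is unused, so it never hides or removes screens.
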(event EventBeginPlay
  (Private|CheackMobile)
  (Private|StartUI))

(event Collision|EventActorBeginOverlap
  (params (OtherActor :type Actor%20Object%20Reference)))

(event EventTick
  (params (DeltaSeconds :type Float%20%28single-precision%29)))

(fn ConstructionScript)

(fn StartUI
  (bind _array_element (Utilities|Array|ForEachLoopwithBreak (Variables|Default|GetScreenConfigs))
    (:LoopBody
      (if (.isstart _array_element)
        (Private|ToggleUI (.screentype _array_element) false)))))

(fn CheackMobile
  (bind _returnvalue (Game|GetPlatformName))
  (Development|PrintString _returnvalue)
  (switch string _returnvalue
    (:Android
      (Private|ToggleUI "NewEnumerator2" true))))

(fn ToggleUI
  (params (ScreenType :type ScreenType%20Enum :default "NewEnumerator0") (IsOn :type Boolean))
  (LocalVariables|SetLocalScreenType ScreenType)
  (bind _array_element (Utilities|Array|ForEachLoopwithBreak (Variables|Default|GetScreenConfigs))
    (:LoopBody
      (if (Utilities|Enum|Equal(Enum) (.screentype _array_element) (LocalVariables|GetLocalScreenType))
        (bind _returnvalue (UserInterface|CreateWidget (.screen _array_element) (Game|GetPlayerController 0)))
        (UserInterface|Viewport|AddtoViewport _returnvalue 0)))))